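; Lobby game mode for the waiting lobby, hosting a dedicated Advanced Sessions session and cleaning it up once empty.
; Login and logout maintain the list of lobby controllers and push its count to GS_Lobby.
; The first login starts a looping timer that, when no players remain, requests PlayFab server shutdown, calls ShutDown and deletes the lobby.
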(event `self.ReceiveBeginPlay`
  ;[1 1 1 1 55] Create Dedicated Session
  (if (`KismetSystemLibrary.IsDedicatedServer`)
    (`CreateSessionCallbackProxyAdvanced.CreateAdvancedSession` :`PlayerController` null :`PrivateConnections` 100 :`bIsDedicatedServer` true :`bUsePresence` false :`bUseLobbiesIfAvailable` false
      (:`OnSuccess`
        (`KismetSystemLibrary.PrintString` "Dedicated session created"))
      (:`OnFailure`
        (`KismetSystemLibrary.PrintString` "Could not create dedicated session")))))

(event `self.ReceiveTick`
  (params (DeltaSeconds :type "Float (single-precision)")))

(event `self.K2_PostLogin`
  (params (NewPlayer :type "PlayerController Object Reference"))
  (bind _allpcs (`self.AllPCs`))
  ;[1 1 1 1 55] Server logic
  (`KismetArrayLibrary.Array_Add` _allpcs (cast `/Game/Blueprints/WaitingLobby/PC_Lobby` NewPlayer :!pure true))
  (`KismetSystemLibrary.PrintString` "player joined")
  (`/Game/Blueprints/WaitingLobby/GS_Lobby.UpdateMaxPlayers` (cast `/Game/Blueprints/WaitingLobby/GS_Lobby` (`GameplayStatics.GetGameState`) :!pure true) (`KismetArrayLibrary.Array_Length` _allpcs))
  (`/Engine/EditorBlueprintResources/StandardMacros.DoOnce` false
    (:`Completed`
      (bind _returnvalue (`KismetSystemLibrary.K2_SetTimerDelegate` (delegate `CheckPlayers`) 10.0 true))
      (set `self.CheckPlayersTimerHandle` _returnvalue))))

(event `CheckPlayers`
  ;[1 1 1 1 55] Server logic
  (if (< (`KismetArrayLibrary.Array_Length` (`self.AllPCs`)) 1)
    (`|ExecutionSequence`
      (:`then_0`
        (`PlayFabMultiplayerAPI.ShutdownMultiplayerServer` (make `MultiplayerShutdownMultiplayerServerRequest` null (`self.SessionID`)) (`|CreateDelegate` :!event `ShutdownSuccess`) (`|CreateDelegate` :!event `MyThirdPersonGameMode_AutoGenFunc`)))
      (:`then_1`
        (`ShutDownDS.ShutDown`))
      (:`then_2`
        (`PlayFabMultiplayerAPI.DeleteLobby` (make `MultiplayerDeleteLobbyRequest` null (`self.Lobby Id`)) (delegate `DeleteLobbySuccess`) (`|CreateDelegate` :!event `MyThirdPersonGameMode_AutoGenFunc`))))))

(event `DeleteLobbySuccess`
  (params (result :type "MultiplayerLobbyEmptyResult Structure") (customData :type "Object Object Reference"))
  ;[1 1 1 1 55] Server logic
  (`KismetSystemLibrary.PrintString` "Lobby Deleted"))

(event `self.K2_OnLogout`
  (params (ExitingController :type "Controller Object Reference"))
  (bind _allpcs (`self.AllPCs`))
  ;[1 1 1 1 55] Server logic
  (`KismetArrayLibrary.Array_RemoveItem` _allpcs (cast `/Game/Blueprints/WaitingLobby/PC_Lobby` ExitingController :!pure true))
  (`/Game/Blueprints/WaitingLobby/GS_Lobby.UpdateMaxPlayers` (cast `/Game/Blueprints/WaitingLobby/GS_Lobby` (`GameplayStatics.GetGameState`) :!pure true) (`KismetArrayLibrary.Array_Length` _allpcs)))

(event `ShutdownSuccess`
  (params (result :type "MultiplayerEmptyResponse Structure") (customData :type "Object Object Reference"))
  ;[1 1 1 1 55] Server logic
  (`KismetSystemLibrary.PrintString` "Shutdown Success"))

(fn `MyThirdPersonGameMode_AutoGenFunc`
  (params (error :type "PlayFabError Structure") (customData :type "Object Object Reference"))
  (bind (_haserror _errorcode _errorname _errormessage _errordetails) (break `PlayFabError` error))
  (`KismetSystemLibrary.PrintString` (`KismetStringLibrary.Concat_StrStr` _errorname _errormessage _errordetails)))

(fn `UserConstructionScript`)