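; Lobby GameState that tracks how many players are ready and launches the match on Level1 once enough are.
; UpdatePlayerCount adjusts ReadyCount; reaching MaxPlayers starts a server-side looping one-second timer that counts down, or resets if readiness drops.
; Countdown UI updates go only through player controller 0's PC_Lobby.
; At zero it saves the player count to BP_GameInstance, creates loading screens, sets each PlayerState's level and calls servertravel.
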(event `UpdatePlayerCount`
  (params (`Increment?` :type Boolean))
  ;[1 1 1 1 55] UpdatePlayerCount
  (`|ExecutionSequence`
    (:`then_0`
      (`self.UpdateValue` `Increment?`))
    (:`then_1`
      (if (>= (`self.ReadyCount`) (`self.MaxPlayers`))
        (`self.ServerStartCountdown`)))))

(event `ServerStartCountdown`
  ;[1 1 1 1 55] Start Countdown
  (if (`KismetSystemLibrary.IsServer`)
    (bind _returnvalue (`KismetSystemLibrary.K2_SetTimerDelegate` (delegate `CheckIfAllReady`) 1.0 true))
    (set `self.CountdownTimer` _returnvalue)))

(event `CheckIfAllReady`
  (bind _countdown (`self.Countdown`))
  ;[1 1 1 1 55] Start Countdown
  (if (>= (`self.ReadyCount`) (`self.MaxPlayers`))
    (if (>= (`self.MaxPlayers`) (`self.MinPlayersRequiredToStart`))
      (bind _output_get (set `self.Countdown` (- _countdown 1.0)))
      (`self.UpdateCountdown` _output_get)
      (if (<= _countdown 0.0)
        ;[1 1 1 1 55] Server Travel
        (`/Game/Blueprints/GameInstance/BPI_GameInstance.SetPlayerCountInCurrentGame` (cast `/Game/Blueprints/GameInstance/BP_GameInstance` (`GameplayStatics.GetGameInstance`) :!pure true) (`self.ReadyCount`))
        (for _array_element (`GameStateBase.PlayerArray` (`GameplayStatics.GetGameState`))
          (`/Game/Blueprints/Common/PC_Base.CreateLoadingScreen` (cast `/Game/Blueprints/Common/PC_Base` (`PlayerState.GetPlayerController` _array_element) :!pure true))
          (bind _asps_base (cast `/Game/Blueprints/Common/PS_Base` (`Pawn.PlayerState` (`PlayerState.GetPawn` _array_element))))
          (set `/Game/Blueprints/Common/PS_Base.CurrentLevel` 1 _asps_base))
        (`KismetSystemLibrary.ExecuteConsoleCommand` "servertravel Level1" null)))
    (else
      (set `self.Countdown` 6.0)
      (`self.ResetCountdown`)
      (`KismetSystemLibrary.K2_ClearAndInvalidateTimerHandle` (`self.CountdownTimer`)))))

(event `UpdateCountdown`
  (params (TimerVal :type "Float (double-precision)"))
  (bind _aspc_lobby (cast `/Game/Blueprints/WaitingLobby/PC_Lobby` (`GameplayStatics.GetPlayerController` 0) :!pure true))
  ;[1 1 1 1 55] Update Countdown Value
  (`/Engine/EditorBlueprintResources/StandardMacros.IsValid` _aspc_lobby
    (:`Is Valid`
      (`/Game/Blueprints/WaitingLobby/PC_Lobby.UpdateCountdownEvent` _aspc_lobby TimerVal))))

(event `ResetCountdown`
  ;[1 1 1 1 55] Update Countdown Value
  (`/Game/Blueprints/WaitingLobby/PC_Lobby.SetVisibilityUIEvent` (cast `/Game/Blueprints/WaitingLobby/PC_Lobby` (`GameplayStatics.GetPlayerController` 0) :!pure true) false))

(fn `OnRep_ReadyCount`)

(fn `UpdateMaxPlayers`
  (params (MaxPlayers :type Integer))
  (set `self.MaxPlayers` MaxPlayers))

(fn `UpdateValue`
  (params (Condition :type Boolean))
  (bind _readycount (`self.ReadyCount`))
  (if Condition
    (`/Engine/EditorBlueprintResources/StandardMacros.IncrementInt` _readycount)
    (else
      (bind _result (`/Engine/EditorBlueprintResources/StandardMacros.DecrementInt` _readycount)
        (:`  `
          (set `self.ReadyCount` (`KismetMathLibrary.Clamp` _result 0 30)))))))

(fn `UserConstructionScript`)