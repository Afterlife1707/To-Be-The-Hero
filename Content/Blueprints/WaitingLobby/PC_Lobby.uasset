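; Player controller for the waiting lobby, handling character selection UI, ready toggling and countdown display.
; On begin play the local controller sends the GameInstance's session ID to GM_Lobby, which keeps the first, and non-dedicated instances open character selection.
; CreateWaitingWidget switches to the lobby HUD and game input.
; The F key flips PS_Base readiness, updates the HUD and forwards it through SR_Ready to GS_Lobby's player count.
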(event `self.ReceiveBeginPlay`
  ;[1 1 1 1 55] Init
  (`|ExecutionSequence`
    (:`then_0`
      (`self.SendSessionInfo`))
    (:`then_1`
      (if (not (`KismetSystemLibrary.IsDedicatedServer`))
        (bind _returnvalue (`|CreateWidget` "/Game/Widgets/WaitingLobby/WBP_CharacterSelection.WBP_CharacterSelection_C" null self))
        (`UserWidget.AddToViewport` _returnvalue 0)
        (`WidgetBlueprintLibrary.SetInputMode_UIOnlyEx` self _returnvalue "LockAlways")
        (set `self.bShowMouseCursor` true)))))

(event `SR_UpdatePlayerCount`
  ;[1 1 1 1 55] Init
  (`/Game/Widgets/WaitingLobby/WBP_WaitingLobby.UpdateCurrentPlayerCountText` (`self.LobbyWidget`)))

(event `Key|F`
  (params (Key :type "Key Structure"))
  ;[1 1 1 1 45] Toggle Ready
  (:`Pressed`
    (`self.ToggleReady`)))

(event `ToggleReady`
  (bind _asps_base (cast `/Game/Blueprints/Common/PS_Base` (`self.PlayerState`) :!pure true))
  (bind _bisready (`/Game/Blueprints/Common/PS_Base.bIsReady` _asps_base))
  ;[1 1 1 1 45] Toggle Ready
  (bind _output_get (set `/Game/Blueprints/Common/PS_Base.bIsReady` (not _bisready) _asps_base))
  (`/Game/Widgets/WaitingLobby/WBP_WaitingLobby.UpdateReadyUI` (`self.LobbyWidget`) _output_get)
  (`self.SR_Ready` _bisready))

(event `SR_Ready`
  (params (isReady :type Boolean))
  ;[1 1 1 1 45] Toggle Ready
  (bind _output_get (set `/Game/Blueprints/Common/PS_Base.bIsReady` isReady (cast `/Game/Blueprints/Common/PS_Base` (`self.PlayerState`) :!pure true)))
  (`/Game/Blueprints/WaitingLobby/GS_Lobby.UpdatePlayerCount` (cast `/Game/Blueprints/WaitingLobby/GS_Lobby` (`GameplayStatics.GetGameState`) :!pure true) _output_get))

(event `UpdateCountdownEvent`
  (params (TimerVal :type "Float (double-precision)"))
  (bind _lobbywidget (`self.LobbyWidget`))
  ;[1 1 1 1 45] Toggle Ready
  (`/Engine/EditorBlueprintResources/StandardMacros.IsValid` _lobbywidget
    (:`Is Valid`
      (`/Game/Widgets/WaitingLobby/WBP_WaitingLobby.SetVisibilityCountdownUI` _lobbywidget true)
      (`/Game/Widgets/WaitingLobby/WBP_WaitingLobby.UpdateCountdownValue` _lobbywidget TimerVal))))

(event `SetVisibilityUIEvent`
  (params (bIsVisible :type Boolean))
  (bind _lobbywidget (`self.LobbyWidget`))
  ;[1 1 1 1 45] Toggle Ready
  (`/Engine/EditorBlueprintResources/StandardMacros.IsValid` _lobbywidget
    (:`Is Valid`
      (`/Game/Widgets/WaitingLobby/WBP_WaitingLobby.SetVisibilityCountdownUI` _lobbywidget bIsVisible))))

(event `SendSessionIdToServer`
  (params (SessionID :type String))
  ;[1 1 1 1 34] Session ID
  (bind _asgm_lobby (cast `/Game/Blueprints/WaitingLobby/GM_Lobby` (`GameplayStatics.GetGameMode`)))
  (if (`KismetStringLibrary.IsEmpty` (`/Game/Blueprints/WaitingLobby/GM_Lobby.SessionID` _asgm_lobby))
    (set `/Game/Blueprints/WaitingLobby/GM_Lobby.SessionID` SessionID _asgm_lobby)))

(fn `CreateWaitingWidget`
  (bind _returnvalue (`|CreateWidget` "/Game/Widgets/WaitingLobby/WBP_WaitingLobby.WBP_WaitingLobby_C" (`GameplayStatics.GetPlayerController` 0)))
  (bind _output_get (set `self.LobbyWidget` _returnvalue))
  (`UserWidget.AddToViewport` _output_get 0)
  (`WidgetBlueprintLibrary.SetInputMode_GameOnly` self)
  (set `self.bShowMouseCursor` false)
  (`self.SR_UpdatePlayerCount`))

(fn `SendSessionInfo`
  (if (`self.IsLocalPlayerController`)
    (bind _sessionid (message `/Game/Blueprints/GameInstance/BI_GameInstance.GetSessionID` (`GameplayStatics.GetGameInstance`)))
    (`self.SendSessionIDToServer` _sessionid)))

(fn `UserConstructionScript`)