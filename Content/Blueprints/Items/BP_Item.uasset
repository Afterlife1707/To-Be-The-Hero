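; BP_Item is an item Blueprint that knocks back third-person characters its box collision hits, ignoring its instigator.
; On a hit, it casts the other actor to BP_ThirdPersonCharacter and calls that character's SRPlaySound to play the item's sound effect at the character's location.
; It then launches the character along the stored instigator forward vector, scaled by LaunchVelocity and added to existing velocity.
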(event `self.BoxCollision.OnComponentHit`
  (params (HitComponent :type "PrimitiveComponent Object Reference") (OtherActor :type "Actor Object Reference") (OtherComp :type "PrimitiveComponent Object Reference") (NormalImpulse :type "Vector Structure") (Hit :type "HitResult Structure (by ref)"))
  (if (!= OtherActor (`self.GetInstigator`))
    (bind _asbp_third_person_character (cast `/Game/Blueprints/BP_ThirdPersonCharacter` OtherActor))
    (`/Game/Blueprints/BP_ThirdPersonCharacter.SR_PlaySound` _asbp_third_person_character (`self.SoundEffect`) (`self.K2_GetActorLocation` _asbp_third_person_character))
    (`Character.LaunchCharacter` _asbp_third_person_character (* (`self.InstigatorForwardVector`) (`self.LaunchVelocity`)) false false)))

(fn `UserConstructionScript`)