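; Player controller that sets up the online session on dedicated servers and passes a session ID to the game mode.
; On BeginPlay, a dedicated server creates an Advanced Sessions session without presence or lobbies.
; A local controller reads the session ID message from the game instance and sends it through SendSessionIdToServer.
; That event stores the ID in MyThirdPersonGameMode only if none is set, so the first ID received sticks.
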(event `self.ReceiveBeginPlay`
  (`|ExecutionSequence`
    (:`then_0`
      (if (`KismetSystemLibrary.IsDedicatedServer`)
        (`CreateSessionCallbackProxyAdvanced.CreateAdvancedSession` :`PlayerController` (`GameplayStatics.GetPlayerController` 0) :`PublicConnections` 30 :`bIsDedicatedServer` true :`bUsePresence` false :`bUseLobbiesIfAvailable` false
          (:`OnSuccess`
            (`KismetSystemLibrary.PrintString` "Session Created"))
          (:`OnFailure`
            (`KismetSystemLibrary.PrintString` "Failed to create session")))))
    (:`then_1`
      (if (`self.IsLocalPlayerController`)
        (bind _sessionid (message `/Game/Blueprints/GameInstance/BI_GameInstance.GetSessionID` (`GameplayStatics.GetGameInstance`)))
        (`self.SendSessionIDToServer` _sessionid)
        (`KismetSystemLibrary.PrintString` "Hello")))))

(event `SendSessionIdToServer`
  (params (SessionID :type String))
  (bind _asmy_third_person_game_mode (cast `/Game/Blueprints/GameLevel/MyThirdPersonGameMode` (`GameplayStatics.GetGameMode`)))
  (if (`KismetStringLibrary.IsEmpty` (`/Game/Blueprints/GameLevel/MyThirdPersonGameMode.SessionID` _asmy_third_person_game_mode))
    (set `/Game/Blueprints/GameLevel/MyThirdPersonGameMode.SessionID` SessionID _asmy_third_person_game_mode)))

(fn `UserConstructionScript`)