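; Main menu player controller that shows the WBP_MainMenu widget and the mouse cursor for the local player on BeginPlay.
; It also contains a PlayFab-style entity token check that fetches a token, validates it and prints success.
; An error event prints the failure details.
; The GetEntityToken call that starts this chain is not wired to run, so the validation is dormant.
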(event `CustomEvent`
  (params (result :type "AuthenticationGetEntityTokenResponse Structure") (customData :type "Object Object Reference"))
  (`PlayFabAuthenticationAPI.ValidateEntityToken` (make `AuthenticationValidateEntityTokenRequest` null (`.EntityToken` (break `AuthenticationGetEntityTokenResponse` result))) (delegate `ValidateEntitySuccess`) (`|CreateDelegate` :!event `ValidationError`)))

(event `ValidateEntitySuccess`
  (params (result :type "AuthenticationValidateEntityTokenResponse Structure") (customData :type "Object Object Reference"))
  (`KismetSystemLibrary.PrintString` "Validation Success"))

(event `self.ReceiveBeginPlay`
  (if (`self.IsLocalController`)
    (bind _returnvalue (`|CreateWidget` "/Game/Widgets/WBP_MainMenu.WBP_MainMenu_C" self))
    (`UserWidget.AddToViewport` _returnvalue 0)
    (set `self.bShowMouseCursor` true)))

(event `ValidationError`
  (params (error :type "PlayFabError Structure") (customData :type "Object Object Reference"))
  (bind (_haserror _errorcode _errorname _errormessage _errordetails) (break `PlayFabError` error))
  (`KismetSystemLibrary.PrintString` (`KismetStringLibrary.Concat_StrStr` _errorname " " _errormessage " " _errordetails)))

(fn `UserConstructionScript`)