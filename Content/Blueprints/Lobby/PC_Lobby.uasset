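; Lobby player controller that shows the waiting-lobby widget and handles the player's ready state.
; Shortly after BeginPlay, the local controller sends the game instance's session ID, which GM_Lobby stores only if it has none.
; F toggles PS_Lobby's ready flag locally, updates the widget, then forwards it through a server event to update GS_Lobby's player count.
; Countdown events drive the widget's timer value and visibility.
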(event `self.ReceiveBeginPlay`
  (`KismetSystemLibrary.Delay` 1.0)
  (`|ExecutionSequence`
    (:`then_0`
      (`self.SendSessionInfo`))
    (:`then_1`
      (if (not (`KismetSystemLibrary.IsDedicatedServer`))
        (bind _returnvalue (`|CreateWidget` "/Game/Widgets/WBP_WaitingLobby.WBP_WaitingLobby_C" (`GameplayStatics.GetPlayerController` 0)))
        (bind _output_get (set `self.LobbyWidget` _returnvalue))
        (`UserWidget.AddToViewport` _output_get 0)))))

(event `Key|F`
  (params (Key :type "Key Structure"))
  (:`Pressed`
    (`self.ToggleReady`)))

(event `ToggleReady`
  (bind _asps_lobby (cast `/Game/Blueprints/Lobby/PS_Lobby` (`self.PlayerState`) :!pure true))
  (bind _bisready (`/Game/Blueprints/Lobby/PS_Lobby.bIsReady` _asps_lobby))
  (bind _output_get (set `/Game/Blueprints/Lobby/PS_Lobby.bIsReady` (not _bisready) _asps_lobby))
  (`/Game/Widgets/WBP_WaitingLobby.UpdateReadyUI` (`self.LobbyWidget`) _output_get)
  (`self.SR_Ready` _bisready))

(event `SR_Ready`
  (params (isReady :type Boolean))
  (bind _output_get (set `/Game/Blueprints/Lobby/PS_Lobby.bIsReady` isReady (cast `/Game/Blueprints/Lobby/PS_Lobby` (`self.PlayerState`) :!pure true)))
  (`/Game/Blueprints/Lobby/GS_Lobby.UpdatePlayerCount` (cast `/Game/Blueprints/Lobby/GS_Lobby` (`GameplayStatics.GetGameState`) :!pure true) _output_get))

(event `UpdateCountdownEvent`
  (params (TimerVal :type "Float (double-precision)"))
  (bind _lobbywidget (`self.LobbyWidget`))
  (`/Engine/EditorBlueprintResources/StandardMacros.IsValid` _lobbywidget
    (:`Is Valid`
      (`/Game/Widgets/WBP_WaitingLobby.SetVisibilityCountdownUI` _lobbywidget true)
      (`/Game/Widgets/WBP_WaitingLobby.UpdateCountdownValue` _lobbywidget TimerVal))))

(event `SetVisibilityUIEvent`
  (params (bIsVisible :type Boolean))
  (bind _lobbywidget (`self.LobbyWidget`))
  (`/Engine/EditorBlueprintResources/StandardMacros.IsValid` _lobbywidget
    (:`Is Valid`
      (`/Game/Widgets/WBP_WaitingLobby.SetVisibilityCountdownUI` _lobbywidget bIsVisible))))

(event `SendSessionIdToServer`
  (params (SessionID :type String))
  ;[1 1 1 1 34] Session ID
  (bind _asgm_lobby (cast `/Game/Blueprints/Lobby/GM_Lobby` (`GameplayStatics.GetGameMode`)))
  (if (`KismetStringLibrary.IsEmpty` (`/Game/Blueprints/Lobby/GM_Lobby.SessionID` _asgm_lobby))
    (set `/Game/Blueprints/Lobby/GM_Lobby.SessionID` SessionID _asgm_lobby)))

(fn `CallUpdateCountdown`)

(fn `SendSessionInfo`
  (if (`self.IsLocalPlayerController`)
    (bind _sessionid (message `/Game/Blueprints/GameInstance/BI_GameInstance.GetSessionID` (`GameplayStatics.GetGameInstance`)))
    (`self.SendSessionIDToServer` _sessionid)))

(fn `UserConstructionScript`)