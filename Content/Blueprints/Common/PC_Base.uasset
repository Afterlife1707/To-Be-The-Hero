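; Base player controller for a multiplayer game with a finish line, handling loading screen, HUD and spectating.
; On BeginPlay it creates the local UI, disables pawn input and reports ready; server-to-multicast RPCs sync readiness and PlayerState character type.
; Tab shows the player list, whose updates retry until the UI exists, and respawns go through GM_BaseLevel.
; When allowed, mouse buttons cycle the camera through player characters still short of the finish.
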(event `CreateLoadingScreen`
  ;[1 1 1 1 55] Loading Screen
  (`self.DisplayLoadingScreen`))

(event `/Game/Blueprints/Common/BPI_LevelTransition.DisplayLoadingScreen`
  ;[1 1 1 1 55] Loading Screen
  (`WidgetLayoutLibrary.RemoveAllWidgets`)
  (`/Engine/EditorBlueprintResources/StandardMacros.IsValid` (`self.WB_LoadScreen`)
    (:`Is Valid`
      _)
    (:`Is Not Valid`
      (bind _returnvalue (`|CreateWidget` "/Game/Widgets/WBP_LoadingScreen.WBP_LoadingScreen_C" self))
      (set `self.WB_LoadScreen` _returnvalue)))
  (`UserWidget.AddToViewport` (`self.WB_LoadScreen`) 0))

(event `self.ReceiveBeginPlay`
  (bind _returnvalue (`GameplayStatics.GetPlayerController` 0))
  ;[1 1 1 1 61] Init
  (`self.InitUI`)
  (if (`self.IsLocalPlayerController`)
    (`self.DisableInput` (`self.K2_GetPawn` _returnvalue) _returnvalue)
    (`self.SR_PlayerReady`)))

(event `Key|Tab`
  (params (Key :type "Key Structure"))
  (bind _uiref (`self.UIRef`))
  ;[1 1 1 1 50] UI
  (:`Pressed`
    (`/Game/Widgets/Common/WBP_UI.ShowPlayers` _uiref true))
  (:`Released`
    (`/Game/Widgets/Common/WBP_UI.ShowPlayers` _uiref false)))

(event `SR_UpdateCharacter`
  (params (CharacterType :type "ECharacterClass Enum" :default "Knight"))
  ;[1 1 1 1 45] Character Selection RPCs
  (`self.ML_UpdateCharacter` CharacterType))

(event `SR_PlayerReady`
  ;[1 1 1 1 55] Player Ready RPCs
  (`self.ML_PlayerReady`))

(event `ML_PlayerReady`
  ;[1 1 1 1 55] Player Ready RPCs
  (set `self.bHasLoaded` true))

(event `ML_UpdateCharacter`
  (params (CharacterType :type "ECharacterClass Enum" :default "Knight"))
  ;[1 1 1 1 45] Character Selection RPCs
  (bind _asps_base (cast `/Game/Blueprints/Common/PS_Base` (`self.PlayerState`)))
  (set `/Game/Blueprints/Common/PS_Base.PS_CharacterType` CharacterType _asps_base))

(event `UpdatePlayerListPC`
  (params (PlayerList :type "Array of /Game/Blueprints/Level1/S_Player Structure"))
  (bind _uiref (`self.UIRef`))
  ;[1 1 1 1 50] UI
  (`/Engine/EditorBlueprintResources/StandardMacros.IsValid` _uiref :!label _label
    (:`Is Valid`
      (`/Game/Widgets/Common/WBP_UI.UpdatePlayers` _uiref PlayerList))
    (:`Is Not Valid`
      (`KismetSystemLibrary.Delay` 0.1)
      (goto _label))))

(event `Key|LeftMouseButton`
  (params (Key :type "Key Structure"))
  ;[1 1 1 1 50] Spectate
  (:`Pressed`
    (if (`self.bCanSpectate`)
      (`self.UpdateSpecatators`)
      (`self.Spectate` true))))

(event `RespawnPawn`
  (params (SpawnTransform :type "Transform Structure") (OldSelf :type "/Game/Blueprints/BP_ThirdPersonCharacter Object Reference"))
  ;[1 1 1 1 45] Request Respawn
  (`/Game/Blueprints/Common/GM_BaseLevel.RespawnRequested` (cast `/Game/Blueprints/Common/GM_BaseLevel` (`GameplayStatics.GetGameMode`) :!pure true) self SpawnTransform OldSelf))

(event `Key|RightMouseButton`
  (params (Key :type "Key Structure"))
  ;[1 1 1 1 50] Spectate
  (:`Pressed`
    (if (`self.bCanSpectate`)
      (`self.UpdateSpecatators`)
      (`self.Spectate` false))))

(fn `CallUpdateCountdown`)

(fn `InitUI`
  (if (`self.IsLocalController`)
    (bind _returnvalue (`|CreateWidget` "/Game/Widgets/Common/WBP_UI.WBP_UI_C"))
    (bind _output_get (set `self.UIRef` _returnvalue))
    (`UserWidget.AddToViewport` _output_get 0)))

(fn `Spectate`
  (params (Prev :type Boolean))
  (locals (NewIdx :type Integer))
  (if (> (`KismetArrayLibrary.Array_Length` (`self.SpectateablePlayers`)) 1)
    (if Prev
      (if (<= (`self.CurrentSpectatingPlayer`) 0)
        (set `local.NewIdx` (`KismetArrayLibrary.Array_LastIndex` (`self.SpectateablePlayers`)))
        (else
          (set `local.NewIdx` (- (`self.CurrentSpectatingPlayer`) 1))))
      (elif (== (`self.CurrentSpectatingPlayer`) (`KismetArrayLibrary.Array_LastIndex` (`self.SpectateablePlayers`)))
        (set `local.NewIdx` 0)
        (else
          (set `local.NewIdx` (+ (`self.CurrentSpectatingPlayer`) 1)))))
    (else
      (set `self.CurrentSpectatingPlayer` 0)))
  (bind _output_get (set `self.CurrentSpectatingPlayer` (`local.NewIdx`)))
  (bind _output (`|GetArrayItem` (`self.SpectateablePlayers`) _output_get))
  (`/Engine/EditorBlueprintResources/StandardMacros.IsValid` _output
    (:`Is Valid`
      (bind _output_get_2 (set `self.CurrentSpectatedPlayer` _output))
      (`self.SetViewTargetWithBlend` _output_get_2 0.5))
    (:`Is Not Valid`
      (set `self.CurrentSpectatingPlayer` -1)
      (set `self.CurrentSpectatedPlayer` null)))
  (return))

(fn `UpdateSpecatators`
  (bind _currentspectatedplayer (`self.CurrentSpectatedPlayer`))
  (`KismetArrayLibrary.Array_Clear` (`self.SpectateablePlayers`))
  (bind _outactors (`GameplayStatics.GetAllActorsOfClass` "/Game/Blueprints/BP_ThirdPersonCharacter.BP_ThirdPersonCharacter_C"))
  (for _array_element _outactors
    (`/Engine/EditorBlueprintResources/StandardMacros.IsValid` _array_element
      (:`Is Valid`
        (if (`Pawn.IsPlayerControlled` _array_element)
          (if (not (`ThirdPersonCharacter.bHasReachedFinishLine` _array_element))
            (`KismetArrayLibrary.Array_Add` (`self.SpectateablePlayers`) _array_element))))))
  (`/Engine/EditorBlueprintResources/StandardMacros.IsValid` _currentspectatedplayer
    (:`Is Valid`
      (set `self.CurrentSpectatingPlayer` (`KismetArrayLibrary.Array_Find` (`self.SpectateablePlayers`) _currentspectatedplayer)))
    (:`Is Not Valid`
      (set `self.CurrentSpectatingPlayer` -1))))

(fn `UserConstructionScript`)