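; Base level game mode for multiplayer elimination rounds, running player readiness, respawns, qualification and level travel.
; A delayed, DoOnce-gated Tick polls until pawns exist, then gathers controllers, sets qualifiers at half plus one and triggers the GameState countdown.
; Finisher reports end the round at quota, eliminating an unfinished player, or show game over on the last level or without finishers.
; NextLevel shows loading screens and server-travels.
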(event `self.ReceiveTick`
  (params (DeltaSeconds :type "Float (single-precision)"))
  ;[1 1 1 1 66] Are All players loaded
  (`KismetSystemLibrary.Delay` 2.0)
  (`/Engine/EditorBlueprintResources/StandardMacros.DoOnce` false :!label _label
    (:`Completed`
      (set `self.bReadyToStart` false)
      (for _array_element (`GameStateBase.PlayerArray` (`GameplayStatics.GetGameState`))
        (`/Engine/EditorBlueprintResources/StandardMacros.IsValid` (cast `/Game/Blueprints/BP_ThirdPersonCharacter` (`Controller.K2_GetPawn` (`PlayerState.GetPlayerController` _array_element)) :!pure true)
          (:`Is Valid`
            (set `self.bReadyToStart` true))
          (:`Is Not Valid`
            (set `self.bReadyToStart` false)
            (goto _label :!via `Reset`))))
      (if (`self.bReadyToStart`)
        (`self.StartCountdown`)
        (else
          (goto _label :!via `Reset`))))))

(event `RespawnRequested`
  (params (PlayerController :type "/Game/Blueprints/Common/PC_Base Object Reference") (SpawnTransform :type "Transform Structure") (OldSelf :type "/Game/Blueprints/BP_ThirdPersonCharacter Object Reference"))
  ;[1 1 1 1 52] Respawn
  (`/Engine/EditorBlueprintResources/StandardMacros.IsValid` PlayerController
    (:`Is Valid`
      (`/Engine/EditorBlueprintResources/StandardMacros.IsValid` OldSelf
        (:`Is Valid`
          (`self.K2_DestroyActor` OldSelf))
        (:`Is Not Valid`
          (`KismetSystemLibrary.PrintString` "invalid")))
      (bind _returnvalue (`|SpawnActorFromClass` "/Game/Blueprints/BP_ThirdPersonCharacter.BP_ThirdPersonCharacter_C" SpawnTransform "Undefined" "MultiplyWithRoot" null null))
      (`KismetSystemLibrary.Delay` 0.2)
      (`Controller.Possess` PlayerController _returnvalue)
      (`/Game/Blueprints/BP_ThirdPersonCharacter.Set Up Local` _returnvalue))))

(event `StartCountdown`
  (bind _allpcs (`self.AllPCs`))
  (bind _playerarray (`GameStateBase.PlayerArray` (`GameplayStatics.GetGameState`)))
  ;[1 1 1 1 109] Round Start Countdown
  (for _array_element _playerarray
    (`KismetArrayLibrary.Array_Add` _allpcs (cast `/Game/Blueprints/Common/PC_Base` (`PlayerState.GetPlayerController` _array_element) :!pure true))
    (`self.UpdatePlayerList`)
    (bind _count (`/Game/Blueprints/GameInstance/BPI_GameInstance.GetPlayerCountInCurrentGame` (cast `/Game/Blueprints/GameInstance/BP_GameInstance` (`GameplayStatics.GetGameInstance`) :!pure true)))
    (if (== (`KismetArrayLibrary.Array_Length` _allpcs) _count)
      (`/Engine/EditorBlueprintResources/StandardMacros.DoOnce` false
        (:`Completed`
          (bind _output_get (set `self.QualifiersCount` (+ (/ (`KismetArrayLibrary.Array_Length` _playerarray) 2) 1)))
          (`KismetSystemLibrary.PrintString` (`KismetStringLibrary.Concat_StrStr` "Qualifiers Count : " (`KismetStringLibrary.Conv_IntToString` _output_get)) true true (struct :`G` 0.66 :`B` 1.0 :`A` 1.0) 5.0)
          (`/Game/Blueprints/Common/GS_BaseLevel.Round Start Countdown` (cast `/Game/Blueprints/Common/GS_BaseLevel` (`GameplayStatics.GetGameState`) :!pure true)))))))

(event `self.K2_PostLogin`
  (params (NewPlayer :type "PlayerController Object Reference"))
  ;[1 1 1] wont be called on seamless
)

(event `NextLevel`
  ;[1 1 1 1 66] Next Level
  (for _array_element (`GameStateBase.PlayerArray` (`GameplayStatics.GetGameState`))
    (`/Game/Blueprints/Common/PC_Base.CreateLoadingScreen` (cast `/Game/Blueprints/Common/PC_Base` (`PlayerState.GetPlayerController` _array_element) :!pure true))
    (bind _asps_base (cast `/Game/Blueprints/Common/PS_Base` (`Pawn.PlayerState` (`PlayerState.GetPawn` _array_element))))
    (set `/Game/Blueprints/Common/PS_Base.CurrentLevel` (`self.LevelToTravelTo`) _asps_base))
  (`KismetSystemLibrary.ExecuteConsoleCommand` (`KismetStringLibrary.Concat_StrStr` "servertravel Level" (`KismetStringLibrary.Conv_IntToString` (`self.LevelToTravelTo`))) null))

(fn `GameOver`
  (params (WinnerName :type String))
  (if (== (`self.FinishedPlayersCount`) 0)
    ;[1 1 1 1 40] Game Over Display
    (set `/Game/Blueprints/Common/GS_BaseLevel.bIsGameOver` true (cast `/Game/Blueprints/Common/GS_BaseLevel` (`GameplayStatics.GetGameState`) :!pure true) :!label _label)
    (set `self.CurrentFinisher` WinnerName)
    (for _array_element (`self.AllPCs`)
      (bind _asbp_third_person_character (cast `/Game/Blueprints/BP_ThirdPersonCharacter` (`Controller.K2_GetPawn` _array_element) :!pure true))
      (`/Game/Blueprints/BP_ThirdPersonCharacter.CL_PlayerFinished` _asbp_third_person_character "")
      (if (== (`self.FinishedPlayersCount`) 0)
        (`/Game/Blueprints/BP_ThirdPersonCharacter.CreateGameOverOnClient` _asbp_third_person_character "" true)
        (else
          (`/Game/Blueprints/BP_ThirdPersonCharacter.CreateGameOverOnClient` _asbp_third_person_character (`self.CurrentFinisher`) false))))
    (elif (`self.bIsLastLevel`)
      (goto _label)
      (else
        ;[1 1 1 1 40] Round Over
        (set `self.bIsRoundOver` true)
        (for _array_element_2 (`self.AllPCs`)
          (bind _asps_base (cast `/Game/Blueprints/Common/PS_Base` (`Controller.PlayerState` _array_element_2) :!pure true))
          (if (not (`/Game/Blueprints/Common/PS_Base.bHasFinished` _asps_base))
            (set `MyPlayerState.bQualifiedForNextRound` false _asps_base)
            (`/Game/Blueprints/BP_ThirdPersonCharacter.CL_PlayerFinished` (cast `/Game/Blueprints/BP_ThirdPersonCharacter` (`Controller.K2_GetPawn` _array_element_2) :!pure true) "You Lose")
            (`self.DisableInput` _array_element_2)
            (return)))))))

(fn `Update Player Finish Count`
  (params (FinisherName :type String))
  (if (`self.bIsLastLevel`)
    (`self.GameOver` FinisherName)
    (else
      (bind _output_get (set `self.FinishedPlayersCount` (+ (`self.FinishedPlayersCount`) 1)))
      (if (>= _output_get (`self.QualifiersCount`))
        (`self.GameOver` "")))))

(fn `UpdatePlayerList`
  (`KismetArrayLibrary.Array_Clear` (`self.Players`))
  (for _array_element (`self.AllPCs`)
    (`KismetArrayLibrary.Array_Add` (`self.Players`) (make `/Game/Blueprints/Level1/S_Player` (`KismetTextLibrary.Conv_StringToText` (`PlayerState.GetPlayerName` (`Controller.PlayerState` _array_element))))))
  (for _array_element_2 (`self.AllPCs`)
    (`/Game/Blueprints/Common/PC_Base.UpdatePlayerListPC` _array_element_2 (`self.Players`))))

(fn `UserConstructionScript`)