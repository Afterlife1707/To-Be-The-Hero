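; Base player controller for Level 1 that manages the local HUD, round countdown and respawn requests.
; On BeginPlay it creates WBP_UI, disables pawn input and signals readiness through SR/ML events that set HasLoaded.
; Tick displays the externally set countdown, then restores input with a start sound when it expires.
; It also toggles the player list on Tab, retries list updates until the UI exists, and forwards respawns to GM_Level1.
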(event `self.ReceiveBeginPlay`
  (bind _returnvalue (`GameplayStatics.GetPlayerController` 0))
  ;[1 1 1 1 61] Init
  (`self.InitUI`)
  (if (`self.IsLocalPlayerController`)
    (`self.DisableInput` (`self.K2_GetPawn` _returnvalue) _returnvalue)
    (`self.SR_PlayerReady`)))

(event `SR_PlayerReady`
  (`self.ML_PlayerReady`))

(event `ML_PlayerReady`
  (set `self.bHasLoaded` true))

(event `Key|Tab`
  (params (Key :type "Key Structure"))
  (bind _uiref (`self.UIRef`))
  ;[1 1 1 1 50] UI
  (:`Pressed`
    (`/Game/Widgets/Common/WBP_UI.ShowPlayers` _uiref true))
  (:`Released`
    (`/Game/Widgets/Common/WBP_UI.ShowPlayers` _uiref false)))

(event `self.ReceiveTick`
  (params (DeltaSeconds :type "Float (single-precision)"))
  (bind _returnvalue (`GameplayStatics.GetPlayerController` 0))
  (bind _uiref (`self.UIRef`))
  (bind _countdown (`self.Countdown`))
  ;[1 1 1 1 87] Tick
  (if (`KismetSystemLibrary.IsValid` _uiref)
    (if (<= _countdown 0.0)
      (if (`self.bIsRoundOver`)
        _
        (elif (not (`self.bStartSoundPlayed`))
          (`self.EnableInput` (`self.K2_GetPawn` _returnvalue) _returnvalue)
          (`GameplayStatics.PlaySound2D` "/Game/Audio/startSound.startSound" 1.0 1.0 0.0 null null)
          (set `self.bStartSoundPlayed` true)
          (`/Game/Widgets/Common/WBP_UI.UpdateTimerCountdown` _uiref 0.0 "")))
      (else
        (if (`self.bIsRoundOver`)
          (set `self.Text to Display` "Game Over \n")
          (else
            (set `self.Text to Display` "Game Starting in ")))
        (`/Game/Widgets/Common/WBP_UI.UpdateTimerCountdown` _uiref _countdown (`self.Text to Display`))))))

(event `UpdatePlayerListPC`
  (params (PlayerList :type "Array of /Game/Blueprints/Level1/S_Player Structure"))
  (bind _uiref (`self.UIRef`))
  ;[1 1 1 1 50] UI
  (`/Engine/EditorBlueprintResources/StandardMacros.IsValid` _uiref :!label _label
    (:`Is Valid`
      (`/Game/Widgets/Common/WBP_UI.UpdatePlayers` _uiref PlayerList))
    (:`Is Not Valid`
      (`KismetSystemLibrary.Delay` 0.1)
      (goto _label))))

(event `RespawnPawn`
  (params (SpawnTransform :type "Transform Structure"))
  ;[1 1 1 1 45] Request Respawn
  (`/Game/Blueprints/Common/GM_BaseLevel.RespawnRequested` (cast `/Game/Blueprints/Level1/GM_Level1` (`GameplayStatics.GetGameMode`) :!pure true) self SpawnTransform))

(fn `CallUpdateCountdown`)

(fn `InitUI`
  (if (`self.IsLocalController`)
    (bind _returnvalue (`|CreateWidget` "/Game/Widgets/Common/WBP_UI.WBP_UI_C"))
    (bind _output_get (set `self.UIRef` _returnvalue))
    (`UserWidget.AddToViewport` _output_get 0)))

(fn `UserConstructionScript`)