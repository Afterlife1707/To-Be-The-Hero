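; GS_BaseLevel is a level game state that runs the round flow: start countdown, round timer and next-round countdown.
; Each countdown is a RepNotify loop: a delayed decrement fires its OnRep, which on authority schedules the next tick or phase.
; Round start enables player input and plays a sound; round end, by timeout or GM_BaseLevel's flag, leads to NextLevel.
; BeginPlay also caches all BP_SpawnPoint actors.
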(event `self.ReceiveBeginPlay`
  ;[1 1 1 1 29] Save Spawn points
  (bind _outactors (`GameplayStatics.GetAllActorsOfClass` "/Game/Blueprints/Common/BP_SpawnPoint.BP_SpawnPoint_C"))
  (set `self.SpawnPoints` _outactors))

(event `Round Start Countdown`
  ;[1 1 1 1 55] Round Start Countdown
  (`KismetSystemLibrary.Delay` 1.0)
  (set `self.RoundStartCountdown` (- (`self.RoundStartCountdown`) 1)))

(event `EnableInputForAllPlayers`
  (bind _returnvalue (`GameplayStatics.GetPlayerController` 0))
  ;[1 1 1 1 55] Enable Input On Round Start
  (`self.EnableInput` (`Controller.K2_GetPawn` _returnvalue) _returnvalue)
  (`GameplayStatics.PlaySound2D` "/Game/Audio/FX/startSound.startSound" 1.0 1.0 0.0 null null)
  (set `self.RoundTimerCountdown` 300))

(event `RoundTimer`
  ;[1 1 1 1 61] Round Timer
  (`KismetSystemLibrary.Delay` 1.0)
  (set `self.RoundTimerCountdown` (- (`self.RoundTimerCountdown`) 1)))

(event `NextRoundStartCountdown`
  ;[1 1 1 1 55] Next Round Start Countdown
  (`KismetSystemLibrary.Delay` 1.0)
  (set `self.NextRoundCountdown` (- (`self.NextRoundCountdown`) 1)))

(fn `OnRep_NextRoundCountdown`
  (`/Engine/EditorBlueprintResources/ActorMacros.Switch Has Authority`
    (:`Authority`
      (if (<= (`self.NextRoundCountdown`) 0)
        (`/Game/Blueprints/Common/GM_BaseLevel.NextLevel` (cast `/Game/Blueprints/Common/GM_BaseLevel` (`GameplayStatics.GetGameMode`) :!pure true))
        (else
          (`self.NextRoundStartCountdown`))))))

(fn `OnRep_RoundStartCountdown`
  (`/Engine/EditorBlueprintResources/ActorMacros.Switch Has Authority`
    (:`Authority`
      (if (<= (`self.RoundStartCountdown`) 0)
        (`self.EnableInputForAllPlayers`)
        (`self.RoundTimer`)
        (else
          (`self.Round Start Countdown`))))))

(fn `OnRep_RoundTimerCountdown`
  (bind _asgm_base_level (cast `/Game/Blueprints/Common/GM_BaseLevel` (`GameplayStatics.GetGameMode`) :!pure true))
  (`/Engine/EditorBlueprintResources/ActorMacros.Switch Has Authority`
    (:`Authority`
      (if (`/Game/Blueprints/Common/GM_BaseLevel.bIsRoundOver` _asgm_base_level)
        (set `self.bIsRoundOver` true)
        (`self.NextRoundStartCountdown` :!label _label)
        (elif (<= (`self.RoundTimerCountdown`) 0)
          (`/Game/Blueprints/Common/GM_BaseLevel.GameOver` _asgm_base_level)
          (goto _label)
          (else
            (`self.RoundTimer`)))))))

(fn `UserConstructionScript`)