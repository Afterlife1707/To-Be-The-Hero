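; Lobby game state for Level1 that tracks how many players are ready and server-travels to TestingMap when a countdown ends.
; Ready count changes start a looping one-second server timer once the count reaches MaxPlayers.
; Each tick pushes the countdown to player controller 0's PC_Lobby, or resets it, hides the UI and clears the timer if readiness drops.
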(event `self.ReceiveBeginPlay`)

(event `UpdatePlayerCount`
  (params (`Increment?` :type Boolean))
  (`|ExecutionSequence`
    (:`then_0`
      (`self.UpdateValue` `Increment?`))
    (:`then_1`
      (if (>= (`self.ReadyCount`) (`self.MaxPlayers`))
        (`self.ServerStartCountdown`)))))

(event `ServerStartCountdown`
  (if (`KismetSystemLibrary.IsServer`)
    (bind _returnvalue (`KismetSystemLibrary.K2_SetTimerDelegate` (delegate `CheckIfAllReady`) 1.0 true))
    (set `self.CountdownTimer` _returnvalue)))

(event `CheckIfAllReady`
  (bind _countdown (`self.Countdown`))
  (if (>= (`self.ReadyCount`) (`self.MaxPlayers`))
    (bind _output_get (set `self.Countdown` (- _countdown 1.0)))
    (`self.UpdateCountdown` _output_get)
    (if (<= _countdown 0.0)
      (`KismetSystemLibrary.ExecuteConsoleCommand` "servertravel TestingMap" null))
    (else
      (set `self.Countdown` 6.0)
      (`self.ResetCountdown`)
      (`KismetSystemLibrary.K2_ClearAndInvalidateTimerHandle` (`self.CountdownTimer`)))))

(event `UpdateCountdown`
  (params (TimerVal :type "Float (double-precision)"))
  (bind _aspc_lobby (cast `/Game/Blueprints/Lobby/PC_Lobby` (`GameplayStatics.GetPlayerController` 0) :!pure true))
  (`/Engine/EditorBlueprintResources/StandardMacros.IsValid` _aspc_lobby
    (:`Is Valid`
      (`/Game/Blueprints/Lobby/PC_Lobby.UpdateCountdownEvent` _aspc_lobby TimerVal))))

(event `ResetCountdown`
  (`/Game/Blueprints/Lobby/PC_Lobby.SetVisibilityUIEvent` (cast `/Game/Blueprints/Lobby/PC_Lobby` (`GameplayStatics.GetPlayerController` 0) :!pure true) false))

(fn `OnRep_ReadyCount`)

(fn `UpdateValue`
  (params (Condition :type Boolean))
  (bind _readycount (`self.ReadyCount`))
  (if Condition
    (`/Engine/EditorBlueprintResources/StandardMacros.IncrementInt` _readycount)
    (else
      (bind _result (`/Engine/EditorBlueprintResources/StandardMacros.DecrementInt` _readycount)
        (:`  `
          (set `self.ReadyCount` (`KismetMathLibrary.Clamp` _result 0 30)))))))

(fn `UserConstructionScript`)