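; Spike trap prop that animates on a repeating timer and reacts to the third-person character.
; A looping timer started on BeginPlay drives a FlipFlop that plays the Trap animation forward or in reverse, updating IsActive after a short delay.
; Overlap of the Trap by the character plays the hide animation once, regardless of IsActive.
; IsActive is read only by unconnected debug prints, and no damage is applied here.
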(event `AlternateSpikes`
  (bind _trap (`self.Trap`))
  (`/Engine/EditorBlueprintResources/StandardMacros.FlipFlop`
    (:`A`
      (`SkeletalMeshComponent.SetPlayRate` _trap 1.0)
      (`SkeletalMeshComponent.Play` _trap false)
      (`KismetSystemLibrary.Delay` 0.3)
      (set `self.bIsActive` true))
    (:`B`
      (`SkeletalMeshComponent.SetPlayRate` _trap -1.0)
      (`SkeletalMeshComponent.Play` _trap false)
      (`KismetSystemLibrary.Delay` 0.8)
      (set `self.bIsActive` false))))

(event `self.ReceiveBeginPlay`
  (`KismetSystemLibrary.K2_SetTimerDelegate` (delegate `AlternateSpikes`) 2.0 true))

(event `self.ReceiveTick`
  (params (DeltaSeconds :type "Float (single-precision)")))

(event `self.Trap.OnComponentBeginOverlap`
  (params (OverlappedComponent :type "PrimitiveComponent Object Reference") (OtherActor :type "Actor Object Reference") (OtherComp :type "PrimitiveComponent Object Reference") (OtherBodyIndex :type Integer) (bFromSweep :type Boolean) (SweepResult :type "HitResult Structure (by ref)"))
  (cast `/Game/Blueprints/BP_ThirdPersonCharacter` OtherActor)
  (`SkeletalMeshComponent.PlayAnimation` (`self.Trap`) "/Game/Props/SpikeWithAnim/SpikeTrap_HideAnimation_Anim.SpikeTrap_HideAnimation_Anim" false))

(fn `UserConstructionScript`)