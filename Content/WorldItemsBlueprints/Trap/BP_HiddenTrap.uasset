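; Hidden trap actor that springs when the player's third-person character enters its Radius overlap component.
; The overlap plays the Trap animation forward and sets IsActive, then after a short delay plays it in reverse via a negative play rate.
; IsActive clears after a further delay to allow for retraction; this Blueprint only sets the flag and applies no damage itself.
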(event `self.Radius.OnComponentBeginOverlap`
  (params (OverlappedComponent :type "PrimitiveComponent Object Reference") (OtherActor :type "Actor Object Reference") (OtherComp :type "PrimitiveComponent Object Reference") (OtherBodyIndex :type Integer) (bFromSweep :type Boolean) (SweepResult :type "HitResult Structure (by ref)"))
  (cast `/Game/Blueprints/BP_ThirdPersonCharacter` OtherActor)
  (`self.EnableTrap`)
  (set `self.bIsActive` true)
  (`KismetSystemLibrary.Delay` 1.5)
  (`self.DisableTrap`)
  (`KismetSystemLibrary.Delay` 0.7)
  (set `self.bIsActive` false))

(fn `DisableTrap`
  (bind _trap (`self.Trap`))
  (`SkeletalMeshComponent.SetPlayRate` _trap -1.0)
  (`SkeletalMeshComponent.Play` _trap false))

(fn `EnableTrap`
  (bind _trap (`self.Trap`))
  (`SkeletalMeshComponent.SetPlayRate` _trap 1.0)
  (`SkeletalMeshComponent.Play` _trap false))

(fn `UserConstructionScript`
  (`parent.UserConstructionScript`))