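; BP_Boulder is a physics boulder that repeatedly relaunches from its spawn point.
; LaunchBoulder zeroes velocity and applies a downward impulse with random sideways force, on X or Y depending on the Level1 flag.
; Overlapping a BP_Checkpoint with its sphere teleports it back, relaunches it and restarts a looping timer.
; That timer acts as a fallback, resetting and relaunching the boulder when no checkpoint is hit in time.
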(event `self.ReceiveBeginPlay`
  (set `self.SpawnPoint` (`self.K2_GetActorLocation`))
  (`self.Launch Boulder`)
  (bind _returnvalue (`KismetSystemLibrary.K2_SetTimer` null "Check Timer" (`self.Time`) true))
  (set `self.HitCheckTimer` _returnvalue))

(event `self.Sphere.OnComponentBeginOverlap`
  (params (OverlappedComponent :type "PrimitiveComponent Object Reference") (OtherActor :type "Actor Object Reference") (OtherComp :type "PrimitiveComponent Object Reference") (OtherBodyIndex :type Integer) (bFromSweep :type Boolean) (SweepResult :type "HitResult Structure (by ref)"))
  (cast `/Game/Blueprints/Common/BP_Checkpoint` OtherActor)
  (set `self.bHasHit` true)
  (`self.K2_SetActorLocation` (`self.SpawnPoint`))
  (`self.Launch Boulder`)
  (`KismetSystemLibrary.K2_ClearAndInvalidateTimerHandle` (`self.HitCheckTimer`))
  (bind _returnvalue (`KismetSystemLibrary.K2_SetTimer` null "Check Timer" (`self.Time`) true))
  (set `self.HitCheckTimer` _returnvalue))

(fn `Check Timer`
  (if (not (`self.bHasHit`))
    (`self.K2_SetActorLocation` (`self.SpawnPoint`))
    (`self.Launch Boulder`)))

(fn `Launch Boulder`
  (locals (Impulse :type "Vector Structure" :default (0.0 0.0 0.0)))
  (bind _staticmeshcomponent (`self.StaticMeshComponent`))
  (bind _returnvalue (`KismetMathLibrary.RandomFloatInRange` (`self.Min`) (`self.Max`)))
  (`PrimitiveComponent.SetPhysicsLinearVelocity` _staticmeshcomponent (0.0 0.0 0.0) false "None")
  (if (`self.Level1`)
    (set `local.Impulse` (`KismetMathLibrary.MakeVector` _returnvalue 0.0 -10000.0))
    (else
      (set `local.Impulse` (`KismetMathLibrary.MakeVector` 0.0 _returnvalue -10000.0))))
  (`PrimitiveComponent.AddImpulse` _staticmeshcomponent (`local.Impulse`) "None" false)
  (set `self.bHasHit` false))

(fn `UserConstructionScript`)