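; BP_Lift2 is a lift actor that moves its static mesh back and forth between two relative positions.
; On BeginPlay it waits a random delay of up to five seconds, so multiple lifts can start out of sync.
; It then loops MoveComponentTo between Pos1 and Pos2 over a Duration variable, pausing briefly at each end.
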(event `self.ReceiveBeginPlay`
  (`KismetSystemLibrary.Delay` (`KismetMathLibrary.RandomFloatInRange` 0.0 5.0))
  (`KismetSystemLibrary.MoveComponentTo` (`self.StaticMesh`) (`self.Pos1`) (struct) false false (`self.Duration`) :!label _label)
  (`KismetSystemLibrary.Delay` 1.0)
  (`KismetSystemLibrary.MoveComponentTo` (`self.StaticMesh`) (`self.Pos2`) (struct) false false (`self.Duration`))
  (`KismetSystemLibrary.Delay` 1.0)
  (goto _label))

(fn `UserConstructionScript`)