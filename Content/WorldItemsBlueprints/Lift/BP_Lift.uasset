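; BP_Lift is a lift that shuttles its static mesh back and forth between two relative positions, Pos1 and Pos2.
; On BeginPlay, a dedicated-server or server check gates the SR_Move event, so only the server starts the motion.
; After an initial delay, the event loops endlessly through two MoveComponentTo moves timed by Duration, pausing briefly after each.
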(event `self.ReceiveBeginPlay`
  (if (or (`KismetSystemLibrary.IsDedicatedServer`) (`KismetSystemLibrary.IsServer`))
    (`self.SR_Move`)))

(event `SR_Move`
  (`KismetSystemLibrary.Delay` 2.0)
  (`KismetSystemLibrary.MoveComponentTo` (`self.StaticMesh`) (`self.Pos1`) (struct) false false (`self.Duration`) :!label _label)
  (`KismetSystemLibrary.Delay` 1.0)
  (`KismetSystemLibrary.MoveComponentTo` (`self.StaticMesh`) (`self.Pos2`) (struct) false false (`self.Duration`))
  (`KismetSystemLibrary.Delay` 1.0)
  (goto _label))

(fn `UserConstructionScript`)