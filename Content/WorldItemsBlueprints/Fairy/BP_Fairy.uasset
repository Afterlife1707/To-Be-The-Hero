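; BP_Fairy is a hostile fairy actor that detects players or mounted horses and shoots BP_FairyBullet projectiles at them.
; On a dedicated server, a looping timer runs a large multi-sphere trace from below the fairy to far ahead, looking for targets.
; FairyShoot starts facing the target, plays a dust sound and spawns an aimed bullet from the throw socket.
; FacePlayer re-calls itself after a tiny delay to keep tracking, drawing debug lines.
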(event `self.ReceiveBeginPlay`
  ;[1 1 1 1 55] Init
  (if (`KismetSystemLibrary.IsDedicatedServer`)
    (`self.StartShoot`)))

(event `StartShoot`
  ;[1 1 1 1 55] Sphere Trace
  (`KismetSystemLibrary.K2_SetTimerDelegate` (delegate `Shoot`) 2.0 true))

(event `Shoot`
  (bind _capsulecomponent (`self.CapsuleComponent`))
  (bind _returnvalue (`SceneComponent.K2_GetComponentLocation` _capsulecomponent))
  ;[1 1 1 1 55] Sphere Trace
  (bind _outhits (`KismetSystemLibrary.SphereTraceMultiForObjects` :`Start` (- _returnvalue (0.0 0.0 1000.0)) :`End` (+ _returnvalue (* (`SceneComponent.GetForwardVector` _capsulecomponent) 8000.0)) :`Radius` 2500.0 :`ObjectTypes` (`self.Object Types`) :`DrawDebugType` "ForDuration"))
  (for _array_element _outhits
    ;[1 1 1] Check if horse or player
    (bind _asbp_horse (cast `/Game/Blueprints/Horse/BP_Horse` (`.HitActor` (`GameplayStatics.BreakHitResult` _array_element)))
      (:`then`
        (if (`HorseThirdPerson.bIsMounted` _asbp_horse)
          ;[1 1 1 1 50] Shoot At Player
          (`self.FairyShoot` _asbp_horse)
          (else
            (bind _asbp_third_person_character (cast `/Game/Blueprints/BP_ThirdPersonCharacter` (`.HitActor` (`GameplayStatics.BreakHitResult` _array_element)) :!label _label))
            (`self.FairyShoot` _asbp_third_person_character))))
      (:`CastFailed`
        (goto _label)))
    (set `self.bIsAttacking` true)
    (break))
  (`KismetSystemLibrary.Delay` 1.0)
  (set `self.bIsAttacking` false))

(event `ML_PlaySound`
  (params (Location :type "Vector Structure"))
  ;[1 1 1 1 50] Shoot At Player
  (`GameplayStatics.PlaySoundAtLocation` "/Game/Audio/FX/fairyDust.fairyDust" Location (struct) 1.0 1.0 0.0 "/Game/Audio/FairyAttenuation.FairyAttenuation" null null null))

(event `FacePlayer`
  (params (Player :type "Actor Object Reference"))
  (bind _returnvalue (`self.K2_GetActorLocation`))
  (bind _returnvalue_2 (`KismetMathLibrary.FindRelativeLookAtRotation` (`KismetMathLibrary.Conv_VectorToTransform` _returnvalue) (`self.K2_GetActorLocation` Player)))
  ;[1 1 1 1 55] FacePlayer
  (`KismetSystemLibrary.DrawDebugLine` _returnvalue (`KismetMathLibrary.Conv_RotatorToVector` _returnvalue_2) (struct :`G` 0.027308 :`B` 1.0 :`A` 1.0) 0.0 5.0)
  (`self.K2_SetActorRotation` _returnvalue_2)
  (`KismetSystemLibrary.Delay` 0.001)
  (`self.FacePlayer` Player))

(fn `FairyShoot`
  (params (Player :type "Actor Object Reference"))
  (bind _returnvalue (`self.K2_GetActorLocation`))
  (`self.FacePlayer` Player)
  (`self.ML_PlaySound` _returnvalue)
  (`|SpawnActorFromClass` "/Game/WorldItemsBlueprints/Fairy/BP_FairyBullet.BP_FairyBullet_C" (`KismetMathLibrary.MakeTransform` (`SceneComponent.GetSocketLocation` (`self.Mesh`) "throwSocket") (`KismetMathLibrary.FindRelativeLookAtRotation` (`KismetMathLibrary.Conv_VectorToTransform` _returnvalue) (`self.K2_GetActorLocation` Player))) "AlwaysSpawn" "MultiplyWithRoot" null self))

(fn `UserConstructionScript`)