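; BP_FairyBullet is a fairy projectile that hits third-person player characters and bursts on impact.
; Its Sphere's hit event spawns a half-scale energy blast emitter, then calls DestroyProjectile to remove the actor.
; An overlap with any BP_ThirdPersonCharacter other than the instigator calls SRFairyHit on that character, then follows the same impact path; other overlaps are ignored.
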(event `self.ReceiveBeginPlay`)

(event `self.Sphere.OnComponentHit`
  (params (HitComponent :type "PrimitiveComponent Object Reference") (OtherActor :type "Actor Object Reference") (OtherComp :type "PrimitiveComponent Object Reference") (NormalImpulse :type "Vector Structure") (Hit :type "HitResult Structure (by ref)"))
  (`GameplayStatics.SpawnEmitterAtLocation` "/Game/InfinityBladeEffects/Effects/FX_Ability/Defense/P_EnergyBlast_Impact.P_EnergyBlast_Impact" (`self.K2_GetActorLocation`) (struct) (0.5 0.5 0.5) :!label _label)
  (`self.DestroyProjectile`))

(event `self.Sphere.OnComponentBeginOverlap`
  (params (OverlappedComponent :type "PrimitiveComponent Object Reference") (OtherActor :type "Actor Object Reference") (OtherComp :type "PrimitiveComponent Object Reference") (OtherBodyIndex :type Integer) (bFromSweep :type Boolean) (SweepResult :type "HitResult Structure (by ref)"))
  (if (not (== OtherActor (`self.GetInstigator`)))
    (bind _asbp_third_person_character (cast `/Game/Blueprints/BP_ThirdPersonCharacter` OtherActor))
    (`/Engine/EditorBlueprintResources/StandardMacros.IsValid` _asbp_third_person_character
      (:`Is Valid`
        (`/Game/Blueprints/BP_ThirdPersonCharacter.SR_FairyHit` _asbp_third_person_character)
        (goto _label)))))

(fn `UserConstructionScript`)