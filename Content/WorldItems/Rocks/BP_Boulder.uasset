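; BP_Boulder is a physics boulder that repeatedly launches from its spawn point.
; LaunchBoulder zeroes velocity, applies a randomized impulse along negative X with a slight downward push, and clears HasHit.
; Overlapping a BP_Checkpoint with its sphere teleports it back to spawn, relaunches it and restarts the watchdog timer.
; That looping timer resets and relaunches the boulder if no checkpoint is reached within the interval.
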(event `self.ReceiveBeginPlay`
  (set `self.SpawnPoint` (`self.K2_GetActorLocation`))
  (`self.Launch Boulder`)
  (bind _returnvalue (`KismetSystemLibrary.K2_SetTimer` null "Check Timer" 5.0 true))
  (set `self.HitCheckTimer` _returnvalue))

(event `self.Sphere.OnComponentBeginOverlap`
  (params (OverlappedComponent :type "PrimitiveComponent Object Reference") (OtherActor :type "Actor Object Reference") (OtherComp :type "PrimitiveComponent Object Reference") (OtherBodyIndex :type Integer) (bFromSweep :type Boolean) (SweepResult :type "HitResult Structure (by ref)"))
  (cast `/Game/Blueprints/BP_Checkpoint` OtherActor)
  (set `self.bHasHit` true)
  (`self.K2_SetActorLocation` (`self.SpawnPoint`))
  (`self.Launch Boulder`)
  (`KismetSystemLibrary.K2_ClearAndInvalidateTimerHandle` (`self.HitCheckTimer`))
  (bind _returnvalue (`KismetSystemLibrary.K2_SetTimer` null "Check Timer" 5.0 true))
  (set `self.HitCheckTimer` _returnvalue))

(fn `Check Timer`
  (if (not (`self.bHasHit`))
    (`self.K2_SetActorLocation` (`self.SpawnPoint`))
    (`self.Launch Boulder`)
    (`KismetSystemLibrary.PrintString` "timer reset")))

(fn `Launch Boulder`
  (bind _staticmeshcomponent (`self.StaticMeshComponent`))
  (`PrimitiveComponent.SetPhysicsLinearVelocity` _staticmeshcomponent (0.0 0.0 0.0) false "None")
  (`PrimitiveComponent.AddImpulse` _staticmeshcomponent (`KismetMathLibrary.MakeVector` (`KismetMathLibrary.RandomFloatInRange` -300000.0 -250000.0) 0.0 -10000.0) "None" false)
  (set `self.bHasHit` false))

(fn `UserConstructionScript`)