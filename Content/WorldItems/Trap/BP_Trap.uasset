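; BP_Trap is a spike trap world item that cycles between extended and retracted on a looping timer.
; Each timer tick, a FlipFlop either plays the Trap animation forward with a spike sound or plays it in reverse.
; After a short delay on each branch it sets the IsActive flag to match the spike state.
; The overlap event is disabled, so this graph applies no damage itself.
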(event `AlternateSpikes`
  (bind _trap (`self.Trap`))
  (`/Engine/EditorBlueprintResources/StandardMacros.FlipFlop`
    (:`A`
      (`GameplayStatics.PlaySoundAtLocation` "/Game/Audio/spike.spike" (`SceneComponent.K2_GetComponentLocation` _trap) (struct) 1.0 1.0 0.0 (`self.Attenuation Settings`) null null null)
      (`SkeletalMeshComponent.SetPlayRate` _trap 1.0)
      (`SkeletalMeshComponent.Play` _trap false)
      (`KismetSystemLibrary.Delay` 0.4)
      (set `self.bIsActive` true))
    (:`B`
      (`SkeletalMeshComponent.SetPlayRate` _trap -1.0)
      (`SkeletalMeshComponent.Play` _trap false)
      (`KismetSystemLibrary.Delay` 0.9)
      (set `self.bIsActive` false))))

(event `self.ReceiveBeginPlay`
  (`KismetSystemLibrary.K2_SetTimerDelegate` (delegate `AlternateSpikes`) 4.0 true))

(event `self.ReceiveTick`
  (params (DeltaSeconds :type "Float (single-precision)")))

(fn `UserConstructionScript`)